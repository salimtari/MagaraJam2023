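; BP_Sequence drives a cinematic backdrop, apparently for the main menu, using two level sequences.
; On BeginPlay it disables pawn input, starts NewLevelSequence after a short delay, hides the HUD health bar and pause widgets, and shows the cursor.
; The sequence loops by rebinding its finished event to restart.
; MainMenu plays AfterPlay_Sequence, while Unbind removes MainMenu, not the looping Play event, from that finished binding.
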(event Custom|Play
  (CallFunction|Start))

(event Custom|Start
  (bind _lever (Variables|Default|Getlever))
  (Sequencer|Player|Play _lever :!class /Script/MovieScene.MovieSceneSequencePlayer)
  (EventDispatchers|BindEventtoOnFinished _lever (delegate Custom|Play)))

(event Custom|Unbind
  (EventDispatchers|UnbindEventfromOnFinished (Variables|Default|Getlever) (delegate Custom|MainMenu)))

(event Custom|MainMenu
  (bind _returnvalue (Sequencer|Player|CreateLevelSequencePlayer "/Game/AfterPlay_Sequence.AfterPlay_Sequence"))
  (bind _output_get (Variables|Default|SetAfter _returnvalue))
  (Sequencer|Player|Play _output_get :!class /Script/MovieScene.MovieSceneSequencePlayer))

(event EventBeginPlay
  (bind _returnvalue (Game|GetPlayerController 0))
  (bind _returnvalue_2 (HUD|GetHUD _returnvalue))
  (bind _asfirst_person_hud (Utilities|Casting|CastToFirstPersonHUD _returnvalue_2))
  (Input|DisableInput (Game|Player|GetPlayerPawn 0) (Game|GetPlayerController 0))
  (bind _returnvalue_3 (Sequencer|Player|CreateLevelSequencePlayer "/Game/NewLevelSequence.NewLevelSequence"))
  (Variables|Default|Setlever _returnvalue_3)
  (Utilities|FlowControl|Delay 0.5)
  (CallFunction|Start)
  (Widget|SetVisibility (Variables|/Game/FirstPersonBP/Blueprints/FirstPersonHUD.FirstPersonHUD_C|GetHealthBar _asfirst_person_hud) "Hidden")
  (Widget|SetVisibility (Variables|/Game/FirstPersonBP/Blueprints/FirstPersonHUD.FirstPersonHUD_C|GetPause _asfirst_person_hud) "Hidden")
  (Variables|/Script/Engine.PlayerController|SetbShowMouseCursor _returnvalue true))

(event Collision|EventActorBeginOverlap
  (params (OtherActor :type Actor%20Object%20Reference)))

(event EventTick
  (params (DeltaSeconds :type Float%20%28single-precision%29)))

(fn ConstructionScript)