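; Behavior tree task that makes an enemy pawn attack when the player is in range.
; It casts the controlled pawn to BP_EnemyBase and compares its distance to player pawn 0 against that enemy's AttackRange.
; In range, it calls Attack, waits for AttackAnimTime and finishes with success.
; A failed cast or out-of-range player finishes the task with failure immediately.
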(event EventReceiveExecuteAI
  (params (OwnerController :type AI%20Controller%20Object%20Reference) (ControlledPawn :type Pawn%20Object%20Reference))
  (bind _asbp_enemy_base (Utilities|Casting|CastToBP_EnemyBase ControlledPawn)
    (:then
      (if (< (Math|Vector|Distance(Vector) (Transformation|GetActorLocation ControlledPawn) (Transformation|GetActorLocation (Game|Player|GetPlayerPawn 0))) (Variables|/Game/Blueprints/Enemy/BP_EnemyBase.BP_EnemyBase_C|GetAttackRange _asbp_enemy_base))
        (Default|Attack _asbp_enemy_base)
        (Utilities|FlowControl|Delay (Variables|/Game/Blueprints/Enemy/BP_EnemyBase.BP_EnemyBase_C|GetAttackAnimTime _asbp_enemy_base))
        (AI|BehaviorTree|FinishExecute true)
        (else
          (AI|BehaviorTree|FinishExecute false :!label _label))))
    (:CastFailed
      (goto _label))))