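; BP_Type2 is an enemy that makes a one-way charge, hurting the player on contact and itself along with them.
; The Attack event flags it as attacking and raises its walk speed.
; While attacking, a Box overlap with BP_Character damages that character's BPHealth, halts the enemy's movement and applies heavier damage to its own BPHealth.
; Tick prints velocity for debugging, and the attack-reset logic is left unconnected.
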(event OnComponentBeginOverlap(Box)
  (params (OverlappedComponent :type Primitive%20Component%20Object%20Reference) (OtherActor :type Actor%20Object%20Reference) (OtherComp :type Primitive%20Component%20Object%20Reference) (OtherBodyIndex :type Integer) (bFromSweep :type Boolean) (SweepResult :type Hit%20Result%20Structure%20%28by%20ref%29))
  (bind _asbp_character (Utilities|Casting|CastToBP_Character OtherActor))
  (if (Variables|Default|GetInAttack)
    (Default|ManageHealth (Variables|/Game/Blueprints/Player/BP_Character.BP_Character_C|GetBP_Health _asbp_character) false 50)
    (Pawn|Components|CharacterMovement|DisableMovement (Variables|Character|GetCharacterMovement))
    (Variables|/Script/Engine.MovementComponent|SetVelocity (Variables|Character|GetCharacterMovement) "0, 0, 0")
    (Default|ManageHealth (Variables|Default|GetBP_Health) false 100)))

(event EventBeginPlay
  (|CallParentFunction))

(event EventTick
  (params (DeltaSeconds :type Float%20%28single-precision%29))
  (Development|PrintString (Utilities|String|ToString(Vector) (Transformation|GetVelocity)) true true "(R=0.000000,G=0.660000,B=1.000000,A=1.000000)" 0.0))

(event EventAttack
  (Variables|Default|SetInAttack true)
  (Variables|/Script/Engine.CharacterMovementComponent|SetMaxWalkSpeed (Variables|Character|GetCharacterMovement) 6e+02))

(fn ConstructionScript
  (|CallParentFunction))