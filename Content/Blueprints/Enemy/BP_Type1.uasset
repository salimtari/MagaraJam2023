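; BP_Type1 is an enemy Blueprint with a melee-range attack that damages the player character class, BP_Character.
; Attack plays a montage and, on its notify, line-traces forward from the capsule on Visibility, reducing the hit character's BPHealth; without a montage it traces immediately.
; The construction script runs the parent's, then picks a random material type for the enemy and sets its max health.
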(event EventAttack
  (bind _capsulecomponent (Variables|Default|GetCapsuleComponent))
  (bind _attackanim (Variables|Default|GetAttackAnim))
  (bind _returnvalue (Transformation|GetWorldLocation _capsulecomponent))
  (Utilities|IsValid _attackanim
    (:Is%20Valid
      (Animation|Montage|PlayMontage (Variables|Character|GetMesh) _attackanim
        (:OnNotifyBegin
          _)))
    (:Is%20Not%20Valid
      _))
  (bind _outhit (Collision|LineTraceByChannel _returnvalue (+ (* (Math|Vector|GetForwardVector (Transformation|GetWorldRotation _capsulecomponent)) 2.5e+02) _returnvalue) "TraceTypeQuery1" false 0 "None"))
  (bind _asbp_character (Utilities|Casting|CastToBP_Character (.hitactor _outhit)))
  (Default|ManageHealth (Variables|/Game/Blueprints/Player/BP_Character.BP_Character_C|GetBP_Health _asbp_character) false (Variables|Default|GetValue)))

(fn ConstructionScript
  (|CallParentFunction)
  (Variables|Default|SetEnemyTpye (Utilities|Enum|ByteToEnumE_MaterialType (Math|Conversions|ToByte(Integer) (Math|Random|RandomIntegerinRange 0 2))))
  (Default|SetMaxHealth (Variables|Default|GetBP_Health) 20))