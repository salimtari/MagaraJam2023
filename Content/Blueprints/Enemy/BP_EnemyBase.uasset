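; Base enemy Blueprint that tints its sphere by gem type, takes damage and feeds an AI blackboard.
; PawnSensing stores the first seen BP_Character as the Player key, using a DoOnce that resets on other pawns.
; Damage drains BPHealth; death sets the Alive key true and destroys controller and actor, on the death montage's notify or immediately without one.
; Attack is an empty stub, and construction caches the attack animation's length.
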(event OnSeePawn(PawnSensing)
  (params (Pawn :type Pawn%20Object%20Reference))
  (Utilities|FlowControl|DoOnce false :!label _label
    (:Completed
      (bind _asbp_character (Utilities|Casting|CastToBP_Character Pawn)
        (:then
          (AI|Components|Blackboard|SetValueasObject (AI|GetBlackboard (AI|GetAIController self)) (Utilities|Name|MakeLiteralName "Player") _asbp_character))
        (:CastFailed
          (goto _label Reset))))))

(event Custom|Attack)

(event EventBeginPlay
  (bind _sphere (Variables|Default|GetSphere))
  (switch Utilities|FlowControl|Switch|SwitchonE_MaterialType (Variables|Default|GetEnemyTpye)
    (:NewEnumerator0
      (Rendering|Material|SetMaterial _sphere 0 "/Game/Blueprints/M_Area_Inst_2.M_Area_Inst_2"))
    (:NewEnumerator1
      (Rendering|Material|SetMaterial _sphere 0 "/Game/Blueprints/M_Area_Inst.M_Area_Inst"))
    (:NewEnumerator2
      (Rendering|Material|SetMaterial _sphere 0 "/Game/Blueprints/M_Area_Inst_3.M_Area_Inst_3"))))

(event Game|Damage|EventAnyDamage
  (params (Damage :type Float%20%28single-precision%29) (DamageType :type Damage%20Type%20Object%20Reference) (InstigatedBy :type Controller%20Object%20Reference) (DamageCauser :type Actor%20Object%20Reference))
  (bind _self self)
  (bind _deathanim (Variables|Default|GetDeathAnim))
  (bind _returnvalue (AI|GetAIController _self))
  (Default|ManageHealth (Variables|Default|GetBP_Health) false (Math|Float|Truncate Damage))
  (bind _alive (Default|CheckAlive (Variables|Default|GetBP_Health)))
  (if (not _alive)
    (Utilities|IsValid _deathanim
      (:Is%20Valid
        (Animation|Montage|PlayMontage (Variables|Character|GetMesh) _deathanim
          (:OnNotifyBegin
            _)))
      (:Is%20Not%20Valid
        _))
    (AI|Components|Blackboard|SetValueasBool (AI|GetBlackboard _returnvalue) (Utilities|Name|MakeLiteralName "Alive") true)
    (Actor|DestroyActor _returnvalue)
    (Actor|DestroyActor)))

(fn ConstructionScript
  (bind _returnvalue (Animation|GetPlayLength (Variables|Default|GetAttackAnim)))
  (Variables|Default|SetAttackAnimTime _returnvalue))