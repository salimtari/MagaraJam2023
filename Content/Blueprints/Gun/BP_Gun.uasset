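; BP_Gun is a hitscan laser gun whose gem-typed shots damage only enemies of the matching type.
; PrimaryAttack line-traces from the camera along its forward vector, with the far endpoint lowered in Z.
; An NS_Beam Niagara effect spawns at the supplied fire location, ends at the hit or trace endpoint, and is colored by BulletType.
; A hit BP_EnemyBase takes fixed damage when its type equals the bullet's.
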(event Custom|PrimaryAttack
  (params (PlayerREF :type BP%20Character%20Object%20Reference) (BulletType :type E_MaterialType%20Enum :default "NewEnumerator0") (Fire :type Vector))
  (bind _returnvalue (Game|GetPlayerCameraManager 0))
  (bind _returnvalue_2 (Camera|GetCameraLocation _returnvalue))
  (bind _returnvalue_3 (Transformation|GetActorForwardVector _returnvalue))
  (bind _returnvalue_4 (* _returnvalue_3 1e+04))
  (bind _returnvalue_5 (+ _returnvalue_2 _returnvalue_4))
  (bind _returnvalue_6 (- (.z _returnvalue_5) 5e+02))
  (bind _returnvalue_7 (Math|Vector|MakeVector (.x _returnvalue_5) (.y _returnvalue_5) _returnvalue_6))
  (bind _outhit (Collision|LineTraceByChannel _returnvalue_2 _returnvalue_7 "TraceTypeQuery3" false 0 "None"))
  (bind _returnvalue_8 (Niagara|SpawnSystematLocation "/Game/Blueprints/NS_Beam.NS_Beam" Fire (Math|Rotator|FindLookatRotation Fire (Math|Vector|SelectVector (.location _outhit) _returnvalue_7 (.bblockinghit _outhit)))))
  (Utilities|FlowControl|Sequence
    (:then_1
      (Effects|Components|ParticleSystem|SetVectorParameter _returnvalue_8 "LaserEnd" (Math|Vector|SelectVector (.location _outhit) _returnvalue_7 (.bblockinghit _outhit)))
      (switch Utilities|FlowControl|Switch|SwitchonE_MaterialType BulletType
        (:NewEnumerator0
          (Effects|Components|ParticleSystem|SetColorParameter _returnvalue_8 "Color" "(R=0.027013,G=0.000000,B=1.000000,A=1.000000)"))
        (:NewEnumerator1
          (Effects|Components|ParticleSystem|SetColorParameter _returnvalue_8 "Color" "(R=0.666667,G=0.000000,B=0.005441,A=1.000000)"))
        (:NewEnumerator2
          (Effects|Components|ParticleSystem|SetColorParameter _returnvalue_8 "Color" "(R=0.000000,G=0.635417,B=0.082041,A=1.000000)")))
      (bind _asbp_enemy_base (Utilities|Casting|CastToBP_EnemyBase (.hitactor _outhit)))
      (if (Utilities|Enum|Equal(Enum) (Variables|/Game/Blueprints/Enemy/BP_EnemyBase.BP_EnemyBase_C|GetEnemyTpye _asbp_enemy_base) BulletType)
        (Game|Damage|ApplyDamage _asbp_enemy_base 1e+01 0 0)))))

(fn ConstructionScript)