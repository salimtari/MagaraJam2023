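; BP_Health is a Blueprint that stores current and maximum health values behind getter and setter functions.
; ManageHealth either adds or subtracts a value based on a boolean flag, writing the result through SetHealth.
; Only subtraction is clamped between zero and MaxHealth, so additions can push health past the maximum.
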(fn GetHealth
  (return (Variables|Default|GetHealth)))

(fn GetMaxHealth
  (return (Variables|Default|GetMaxHealth)))

(fn SetHealth
  (params (Health :type Integer))
  (Variables|Default|SetHealth Health)
  (return))

(fn SetMaxHealth
  (params (MaxHealth :type Integer))
  (Variables|Default|SetMaxHealth MaxHealth)
  (return))

(fn ManageHealth
  (params (Add? :type Boolean) (Value :type Integer))
  (bind _health (CallFunction|GetHealth))
  (if Add?
    (CallFunction|SetHealth (+ _health Value))
    (else
      (CallFunction|SetHealth (Math|Integer|Clamp(Integer) (- _health Value) 0 (CallFunction|GetMaxHealth)))))
  (return))