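; BP_Boss is a boss enemy that attacks the player and plays a final montage before being destroyed when its health runs out.
; A recursive Pattern loop picks gem throw, kick or close-range attack by player distance and chance, polling a busy flag between attacks.
; Montage notifies spawn random-type gems or run sphere traces that damage the player.
; A counter periodically rerolls GemType, and Tick prints player distance.
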(event Custom|Throw%20Gem
  (bind _mesh (Variables|Character|GetMesh))
  (bind _throwmontage (Variables|Default|GetThrowMontage))
  (bind _returnvalue (Transformation|GetSocketLocation _mesh "RockSlot"))
  ;[1 0.1373 0] RockThrow
  (Variables|Default|SetCondition true)
  (Utilities|IsValid _throwmontage
    (:Is%20Valid
      (Animation|Montage|PlayMontage (Variables|Character|GetMesh) _throwmontage
        (:then
          (Transformation|SetActorRotation (Math|Rotator|FindLookatRotation (Transformation|GetActorLocation) (Transformation|GetActorLocation (Game|Player|GetPlayerPawn 0)))))
        (:OnCompleted
          (Variables|Default|SetCondition false))
        (:OnNotifyBegin
          (Game|SpawnActorfromClass "/Game/Blueprints/BP_Gem.BP_Gem_C" (Math|Transform|MakeTransform _returnvalue (Math|Rotator|FindLookatRotation _returnvalue (Transformation|GetActorLocation (Game|Player|GetPlayerPawn 0))) "1,1,1") "Undefined" 0 (Utilities|Enum|ByteToEnumE_MaterialType (Math|Conversions|ToByte(Integer) (Math|Random|RandomIntegerinRange 0 2))) (Transformation|GetSocketLocation (Variables|Character|GetMesh) "RockSlot") 0))))))

(event Custom|CloseRangeAttack
  (bind _capsulecomponent (Variables|Collision|GetCapsuleComponent))
  (bind _returnvalue (Transformation|GetWorldLocation _capsulecomponent))
  ;[0.03839 0.1943 1] CloseRangeAttack
  (Variables|Default|SetCondition true)
  (AI|AIMoveTo self "0, 0, 0" (Game|Player|GetPlayerPawn 0) 2e+02 false
    (:OnSuccess
      (Animation|Montage|PlayMontage (Variables|Character|GetMesh) "/Game/FirstPersonBP/Character/Mutant/AM_CloseRangeAttack.AM_CloseRangeAttack"
        (:OnCompleted
          (Variables|Default|SetCondition false))
        (:OnNotifyBegin
          (bind _outhits (Collision|MultiSphereTraceByChannel _returnvalue (+ (* (Math|Vector|GetForwardVector (Transformation|GetWorldRotation _capsulecomponent)) 3e+02) _returnvalue) 1.5e+02 "TraceTypeQuery1" false 0 "None"))
          (Utilities|FlowControl|DoOnce false :!label _label
            (:Completed
              (bind _array_element (Utilities|Array|ForEachLoopwithBreak _outhits :!label _label_2)
                (:LoopBody
                  (bind _asbp_character (Utilities|Casting|CastToBP_Character (.hitactor _array_element))
                    (:then
                      (Game|Damage|ApplyDamage _asbp_character 2e+01 0 0)
                      (goto _label_2 Break))
                    (:CastFailed
                      (goto _label Reset))))))))))))

(event Custom|Kick
  (bind _returnvalue (Transformation|GetActorLocation))
  ;[1 1 1] Kick
  (Variables|Default|SetCondition true)
  (AI|AIMoveTo self "0, 0, 0" (Game|Player|GetPlayerPawn 0) 1e+02 false
    (:OnSuccess
      (Animation|Montage|PlayMontage (Variables|Character|GetMesh) "/Game/FirstPersonBP/Character/Mutant/AM_Kick.AM_Kick"
        (:OnCompleted
          (Variables|Default|SetCondition false))
        (:OnNotifyBegin
          (bind _outhits (Collision|MultiSphereTraceByChannel _returnvalue _returnvalue 4e+02 "TraceTypeQuery4" false 0 "ForDuration"))
          (bind _array_element (Utilities|Array|ForEachLoopwithBreak _outhits :!label _label)
            (:LoopBody
              (Utilities|FlowControl|DoOnce false :!label _label_2
                (:Completed
                  (bind _asbp_character (Utilities|Casting|CastToBP_Character (.hitactor _array_element))
                    (:then
                      (Game|Damage|ApplyDamage _asbp_character 25.0 0 0)
                      (goto _label Break))
                    (:CastFailed
                      (goto _label_2 Reset))))))))))))

(event Custom|Pattern
  (bind _returnvalue (Game|Player|GetPlayerPawn 0))
  (bind _returnvalue_2 (Transformation|GetDistanceTo _returnvalue))
  (bind _result (Math|Integer|IncrementInt (Variables|Default|GetCounter))
    (:%20%20
      (if (== _result 5)
        (Variables|Default|SetGemType (Utilities|Enum|ByteToEnumE_MaterialType (Math|Conversions|ToByte(Integer) (Math|Random|RandomIntegerinRange 0 2))))
        (Variables|Default|SetCounter 0)
        (else
          (bind _alive (Default|CheckAlive (Variables|Default|GetBP_Health)))
          (if _alive
            (if (and (< _returnvalue_2 1.5e+03) (> _returnvalue_2 8e+02))
              (if (Math|Random|RandomBool)
                (CallFunction|ThrowGem)
                (else
                  (if (< _returnvalue_2 3e+02) :!label _label
                    (CallFunction|CloseRangeAttack)
                    (else
                      (CallFunction|Kick)))))
              (else
                (goto _label)))
            (if (Variables|Default|GetCondition) :!label _label_2
              (Utilities|FlowControl|Delay 0.2)
              (goto _label_2)
              (else
                (CallFunction|Pattern)))))))))

(event EventTick
  (params (DeltaSeconds :type Float%20%28single-precision%29))
  (Development|PrintString (Utilities|String|ToString(Float) (Transformation|GetDistanceTo (Game|Player|GetPlayerPawn 0))) true true "(R=0.000000,G=0.660000,B=1.000000,A=1.000000)" 0.0))

(event EventBeginPlay
  (CallFunction|Pattern))

(event Game|Damage|EventAnyDamage
  (params (Damage :type Float%20%28single-precision%29) (DamageType :type Damage%20Type%20Object%20Reference) (InstigatedBy :type Controller%20Object%20Reference) (DamageCauser :type Actor%20Object%20Reference))
  (bind _bp_health (Variables|Default|GetBP_Health))
  (Default|ManageHealth _bp_health false (Math|Float|Truncate Damage))
  (bind _alive (Default|CheckAlive _bp_health))
  (if (not _alive)
    (Utilities|FlowControl|DoOnce false
      (:Completed
        (Pawn|Components|CharacterMovement|DisableMovement (Variables|Character|GetCharacterMovement))
        (Animation|Montage|PlayMontage (Variables|Character|GetMesh) "/Game/FirstPersonBP/Character/Mutant/AM_out.AM_out"
          (:OnCompleted
            (Actor|DestroyActor)))))))

(fn ConstructionScript)