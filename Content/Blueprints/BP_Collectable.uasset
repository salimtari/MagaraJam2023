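; BP_Collectable is a gem pickup that sets the player's current weapon type to its GemType.
; Sphere overlap shows the HUD Pickup prompt and enables input, while end overlap reverses both, with paired DoOnce gates re-arming each other.
; Pressing E casts to BP_Character and destroys the gem only if the type differs, otherwise re-arming the key.
; The construction script colors the mesh blue, red or green by GemType.
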(event OnComponentBeginOverlap(Sphere)
  (params (OverlappedComponent :type Primitive%20Component%20Object%20Reference) (OtherActor :type Actor%20Object%20Reference) (OtherComp :type Primitive%20Component%20Object%20Reference) (OtherBodyIndex :type Integer) (bFromSweep :type Boolean) (SweepResult :type Hit%20Result%20Structure%20%28by%20ref%29))
  (bind _returnvalue (Game|GetPlayerController 0))
  (Utilities|FlowControl|DoOnce false
    (:Completed
      (Utilities|FlowControl|Sequence
        (:then_0
          (Widget|SetVisibility (CallFunction|GetPickup) "Visible")
          (Input|EnableInput _returnvalue))
        (:then_1
          (Utilities|FlowControl|DoOnce false) ; enters at Reset
        )))))

(event OnComponentEndOverlap(Sphere)
  (params (OverlappedComponent :type Primitive%20Component%20Object%20Reference) (OtherActor :type Actor%20Object%20Reference) (OtherComp :type Primitive%20Component%20Object%20Reference) (OtherBodyIndex :type Integer))
  (bind _returnvalue (Game|GetPlayerController 0))
  (Utilities|FlowControl|DoOnce false
    (:Completed
      (Utilities|FlowControl|Sequence
        (:then_0
          (Utilities|FlowControl|DoOnce false) ; enters at Reset
        )
        (:then_1
          (Widget|SetVisibility (CallFunction|GetPickup) "Hidden")
          (Input|DisableInput _returnvalue))))))

(event Input|KeyboardEvents|E
  (params (Key :type Key%20Structure :default "None"))
  (bind _gemtype (Variables|Default|GetGemType))
  (:Pressed
    (Utilities|FlowControl|DoOnce false :!label _label
      (:Completed
        (bind _asbp_character (Utilities|Casting|CastToBP_Character (Game|Player|GetPlayerPawn 0))
          (:then
            (if (Utilities|Enum|NotEqual(Enum) _gemtype (Variables|/Game/Blueprints/Player/BP_Character.BP_Character_C|GetCurrentWeaponType _asbp_character))
              (Variables|/Game/Blueprints/Player/BP_Character.BP_Character_C|SetCurrentWeaponType _asbp_character _gemtype)
              (Actor|DestroyActor)
              (else
                (goto _label Reset))))
          (:CastFailed
            (goto _label Reset)))))))

(fn ConstructionScript
  (bind _staticmesh (Variables|Default|GetStaticMesh))
  (switch Utilities|FlowControl|Switch|SwitchonE_MaterialType (Variables|Default|GetGemType)
    (:NewEnumerator0
      (Rendering|Material|SetMaterial _staticmesh 0 "/Game/Geometry/materials/M_BlueGem.M_BlueGem"))
    (:NewEnumerator1
      (Rendering|Material|SetMaterial _staticmesh 0 "/Game/Geometry/materials/M_RedGem.M_RedGem"))
    (:NewEnumerator2
      (Rendering|Material|SetMaterial _staticmesh 0 "/Game/Geometry/materials/M_GreenGem.M_GreenGem"))))

(fn GetPickup
  (return (Variables|/Game/FirstPersonBP/Blueprints/FirstPersonHUD.FirstPersonHUD_C|GetPickup (.AsFirst%20Person%20HUD (Utilities|Casting|CastToFirstPersonHUD (HUD|GetHUD (Game|GetPlayerController 0)))))))