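; BP_Gate is a gate actor that clears a linked gate once every actor from its spawner has been destroyed.
; Shortly after BeginPlay it triggers SpawnerData, records the spawned count and binds each spawned actor's OnDestroyed event.
; Each destruction decrements the counter, and reaching zero destroys OtherGate rather than this actor.
; The box overlap event is empty, so spawning does not depend on entering a trigger.
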(event OnComponentBeginOverlap(Box)
  (params (OverlappedComponent :type Primitive%20Component%20Object%20Reference) (OtherActor :type Actor%20Object%20Reference) (OtherComp :type Primitive%20Component%20Object%20Reference) (OtherBodyIndex :type Integer) (bFromSweep :type Boolean) (SweepResult :type Hit%20Result%20Structure%20%28by%20ref%29)))

(event Custom|ArrangeActor
  (params (DestroyedActor :type Actor%20Object%20Reference))
  (bind _result (Math|Integer|DecrementInt (Variables|Default|GetSpawnedActor))
    (:%20%20
      (if (== _result 0)
        (Actor|DestroyActor (Variables|Default|GetOtherGate))))))

(event EventBeginPlay
  (bind _spawnerdata (Variables|Default|GetSpawnerData))
  (bind _spawneed (Variables|/Game/Blueprints/BP_SpawnerSystem.BP_SpawnerSystem_C|GetSpawneed _spawnerdata))
  (Utilities|FlowControl|Delay 0.2)
  (Default|TriggerSpawn _spawnerdata)
  (Variables|Default|SetSpawnedActor (Utilities|Array|Length _spawneed))
  (for _array_element _spawneed
    (Game|BindEventtoOnDestroyed _array_element (delegate Custom|ArrangeActor))))

(fn ConstructionScript)