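; BP_Gem is a colored gem projectile that launches itself at the player and switches their weapon type on contact.
; On BeginPlay it leads the player's position using velocity and distance over LaunchSpeed, then applies a suggested toss velocity with debug drawing on and a limited lifespan.
; Sphere overlap with BP_Character copies GemType to CurrentWeaponType and destroys the gem.
; The construction script picks the blue, red or green material from GemType.
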(event OnComponentBeginOverlap(Sphere)
  (params (OverlappedComponent :type Primitive%20Component%20Object%20Reference) (OtherActor :type Actor%20Object%20Reference) (OtherComp :type Primitive%20Component%20Object%20Reference) (OtherBodyIndex :type Integer) (bFromSweep :type Boolean) (SweepResult :type Hit%20Result%20Structure%20%28by%20ref%29))
  (bind _asbp_character (Utilities|Casting|CastToBP_Character OtherActor))
  (Variables|/Game/Blueprints/Player/BP_Character.BP_Character_C|SetCurrentWeaponType _asbp_character (Variables|Default|GetGemType))
  (Actor|DestroyActor))

(event EventBeginPlay
  (bind _returnvalue (Game|Player|GetPlayerPawn 0))
  (bind _projectilemovement (Variables|Default|GetProjectileMovement))
  (bind _tossvelocity (Class|GameplayStatics|BlueprintSuggestProjectileVelocity (Variables|Default|GetStart%20Location) (+ (* (Transformation|GetVelocity _returnvalue) (/ (Transformation|GetDistanceTo _returnvalue) (Variables|Default|GetLaunch%20Speed))) (Transformation|GetActorLocation _returnvalue)) (Variables|Default|GetLaunch%20Speed) 0.0 "DoNotTrace" 0.0 false true))
  (Variables|/Script/Engine.MovementComponent|SetVelocity _projectilemovement _tossvelocity)
  (Variables|/Script/Engine.ProjectileMovementComponent|SetbRotationFollowsVelocity _projectilemovement true)
  (Actor|SetLifeSpan 1e+01))

(event Collision|EventActorBeginOverlap
  (params (OtherActor :type Actor%20Object%20Reference)))

(event EventTick
  (params (DeltaSeconds :type Float%20%28single-precision%29)))

(fn ConstructionScript
  (bind _staticmesh (Variables|Default|GetStaticMesh))
  (switch Utilities|FlowControl|Switch|SwitchonE_MaterialType (Variables|Default|GetGemType)
    (:NewEnumerator0
      (Rendering|Material|SetMaterial _staticmesh 0 "/Game/Geometry/materials/M_BlueGem.M_BlueGem"))
    (:NewEnumerator1
      (Rendering|Material|SetMaterial _staticmesh 0 "/Game/Geometry/materials/M_RedGem.M_RedGem"))
    (:NewEnumerator2
      (Rendering|Material|SetMaterial _staticmesh 0 "/Game/Geometry/materials/M_GreenGem.M_GreenGem"))))